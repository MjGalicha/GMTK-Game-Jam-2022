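; BP_TransformingCube is a golf game prop that swaps its static mesh to match the current world theme.
; It starts as the grass mesh, then on Tick polls BP_GolfGameMode's ChangeWorldState flag.
; While the flag is set, a branch chain on CurrentWorldState picks a grass, ice, sand, concrete or whitebox mesh.
; One further state leaves the mesh unchanged, and unexpected values print an error.
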(event `self.ReceiveBeginPlay`
  ;[1 1 1] Change Object at start
  (`self.ChangeToGrass`))

(event `self.ReceiveTick`
  (params (DeltaSeconds :type "Float (single-precision)"))
  ;[1 1 1] Check if world state has changed, if it has changed, run world state change
  (bind _asbp_golf_game_mode (cast `/Game/GolfGame/Blueprints/BP_GolfGameMode` (`GameplayStatics.GetGameMode`)))
  (if (`/Game/GolfGame/Blueprints/BP_GolfGameMode.Change World State` _asbp_golf_game_mode)
    (`self.Change World State`)))

(event `Change World State`
  ;[1 1 1] Run specific state change function
  (bind _asbp_golf_game_mode (cast `/Game/GolfGame/Blueprints/BP_GolfGameMode` (`GameplayStatics.GetGameMode`)))
  (bind _current_world_state (`/Game/GolfGame/Blueprints/BP_GolfGameMode.Current World State` _asbp_golf_game_mode))
  (if (== _current_world_state 2)
    (`self.ChangeToGrass`)
    (elif (== _current_world_state 4)
      (`self.ChangeToIce`)
      (elif (== _current_world_state 6)
        (`self.ChangeToSand`)
        (elif (== _current_world_state 8)
          (`self.ChangeToConcrete`)
          (elif (== _current_world_state 10)
            (`self.ChangeToWhite`)
            (elif (not (== _current_world_state 12))
              (`KismetSystemLibrary.PrintString` "This Shouldn't Happen"))))))))

(fn `ChangeToConcrete`
  (`StaticMeshComponent.SetStaticMesh` (`self.Whitebox_Cube`) "/Game/GolfGame/Assets/Objects/Cube/Concrete_Skateboard.Concrete_Skateboard"))

(fn `ChangeToGrass`
  (`StaticMeshComponent.SetStaticMesh` (`self.Whitebox_Cube`) "/Game/GolfGame/Assets/Objects/Cube/Grass_DogFountain.Grass_DogFountain"))

(fn `ChangeToIce`
  (`StaticMeshComponent.SetStaticMesh` (`self.Whitebox_Cube`) "/Game/GolfGame/Assets/Objects/Cube/Ice_Rock.Ice_Rock"))

(fn `ChangeToSand`
  (`StaticMeshComponent.SetStaticMesh` (`self.Whitebox_Cube`) "/Game/GolfGame/Assets/Objects/Cube/Sand_Rock.Sand_Rock"))

(fn `ChangeToWhite`
  (`StaticMeshComponent.SetStaticMesh` (`self.Whitebox_Cube`) "/Game/GolfGame/Assets/Objects/Cube/Whitebox_Cube.Whitebox_Cube"))

(fn `UserConstructionScript`)