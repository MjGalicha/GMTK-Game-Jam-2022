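; Base golf ball pawn with mouse-driven orbit and zoom, a charged launch, and a random state roll after each shot.
; Holding Space while the ball is stopped builds launch speed, and releasing it fires the ball along the camera yaw.
; When the ball stops, it rolls 1-12: odd results select a matching state, even ones reset to normal.
; The state events are empty stubs in this base.
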(event `InputAxis|Turn Right / Left Mouse`
  (params (AxisValue :type "Float (single-precision)"))
  ;[0.05098 0.05098 0.05098] Camera Input - Mouse
  (`self.AddControllerYawInput` AxisValue))

(event `self.ReceiveTick`
  (params (DeltaSeconds :type "Float (single-precision)"))
  ;[0.07812 0.07812 0.07812] Every Moment - Ball is Stopped
  (if (<= (`KismetMathLibrary.VSize` (`SceneComponent.GetComponentVelocity` (`self.Sphere`))) 0.1)
    (if (`self.canLaunch`)
      (if (`self.isCharging`)
        (set `self.LaunchSpeed` (+ (* DeltaSeconds 3000.0) (`self.LaunchSpeed`))))
      (elif (`self.ballLaunched`)
        (`self.Resolve Roll`)
        (set `self.ballLaunched` false)
        (set `self.canLaunch` true)))))

(event `InputAxis|Look Up / Down Mouse`
  (params (AxisValue :type "Float (single-precision)"))
  ;[0.05098 0.05098 0.05098] Camera Input - Mouse
  (`self.AddControllerPitchInput` AxisValue))

(event `InputAxis|Zoom In / Out Scroll Wheel`
  (params (AxisValue :type "Float (single-precision)"))
  (bind _springarm (`self.SpringArm`))
  ;[0.05098 0.05098 0.05098] Camera Input - Mouse
  (set `SpringArmComponent.TargetArmLength` (+ (`SpringArmComponent.TargetArmLength` _springarm) (* AxisValue (`self.ScrollSpeed`))) _springarm))

(event `Resolve Roll`
  ;[0.07292 0.07292 0.07292] Resolve Dice Rolling
  (bind _output_get (set `self.rolledNumber` (`KismetMathLibrary.RandomIntegerInRange` 1 12)))
  (if (== 1 (mod _output_get 2))
    (set `self.ballState` (`self.rolledNumber`))
    (`self.Change Ball State`)
    (else
      (set `self.ballState` 0)
      (`self.Change Ball State`)))
  (`KismetSystemLibrary.PrintString` (`KismetStringLibrary.Conv_IntToString` (`self.rolledNumber`))))

(event `Change Ball State`
  (bind _ballstate (`self.ballState`))
  ;[0.09896 0.09896 0.09896] Ball State Changing
  (if (== _ballstate 0)
    (`self.Ball State Normal`)
    (elif (== _ballstate 1)
      (`self.Ball State 1`)
      (elif (== _ballstate 3)
        (`self.Ball State 3`)
        (elif (== _ballstate 5)
          (`self.Ball State 5`)
          (elif (== _ballstate 7)
            (`self.Ball State 7`)
            (elif (== _ballstate 9)
              (`self.Ball State 9`)
              (elif (== _ballstate 11)
                (`self.Ball State 11`)
                (else
                  (`KismetSystemLibrary.PrintString` "This Shouldn't Happen"))))))))))

(event `Key|SpaceBar`
  (params (Key :type "Key Structure"))
  ;[0.06771 0.06771 0.06771] Press and Release Space to Launch Ball
  (:`Pressed`
    (set `self.isCharging` true))
  (:`Released`
    (set `self.isCharging` false)
    (if (`self.canLaunch`)
      (`PrimitiveComponent.SetPhysicsLinearVelocity` (`self.Capsule`) (* (`KismetMathLibrary.GetForwardVector` (`KismetMathLibrary.MakeRotator` 0.0 0.0 (.yaw (`self.GetControlRotation`)))) (`self.LaunchSpeed`)) false "None")
      (`PrimitiveComponent.SetPhysicsLinearVelocity` (`self.Sphere`) (* (`KismetMathLibrary.GetForwardVector` (`KismetMathLibrary.MakeRotator` 0.0 0.0 (.yaw (`self.GetControlRotation`)))) (`self.LaunchSpeed`)) false "None"))
    (set `self.LaunchSpeed` 0.0)
    (set `self.ballLaunched` true)
    (set `self.canLaunch` false)))

(event `Ball State 1`
  ;[1 1 1] Set Ball State 1
)

(event `Ball State 3`
  ;[1 1 1] Set Ball State 3
)

(event `Ball State Normal`
  ;[1 1 1] Set Ball State Normal
)

(event `Ball State 5`
  ;[1 1 1] Set Ball State 5
)

(event `Ball State 7`
  ;[1 1 1] Set Ball State 7
)

(event `Ball State 9`
  ;[1 1 1] Set Ball State 9
)

(event `Ball State 11`
  ;[1 1 1] Set Ball State 11
)

(fn `UserConstructionScript`)