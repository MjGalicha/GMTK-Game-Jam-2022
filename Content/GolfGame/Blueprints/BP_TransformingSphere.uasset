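; BP_TransformingSphere is a golf game prop that swaps its static mesh to match the current world state.
; Every tick it polls the ChangeWorldState flag on BP_GolfGameMode, then branches on CurrentWorldState.
; Per-theme functions set the grass, ice, sand, concrete or whitebox mesh on the WhiteboxSphere component.
; One further state leaves the mesh unchanged, and unexpected values print a debug message.
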(event `self.ReceiveTick`
  (params (DeltaSeconds :type "Float (single-precision)"))
  ;[1 1 1] Check if world state has changed, if it has changed, run world state change
  (bind _asbp_golf_game_mode (cast `/Game/GolfGame/Blueprints/BP_GolfGameMode` (`GameplayStatics.GetGameMode`)))
  (if (`/Game/GolfGame/Blueprints/BP_GolfGameMode.Change World State` _asbp_golf_game_mode)
    (`self.Change World State`)))

(event `Change World State`
  ;[1 1 1] Run specific state change function
  (bind _asbp_golf_game_mode (cast `/Game/GolfGame/Blueprints/BP_GolfGameMode` (`GameplayStatics.GetGameMode`)))
  (bind _current_world_state (`/Game/GolfGame/Blueprints/BP_GolfGameMode.Current World State` _asbp_golf_game_mode))
  (if (== _current_world_state 2)
    (`self.ChangeToGrass`)
    (elif (== _current_world_state 4)
      (`self.ChangeToIce`)
      (elif (== _current_world_state 6)
        (`self.ChangeToSand`)
        (elif (== _current_world_state 8)
          (`self.ChangeToConcrete`)
          (elif (== _current_world_state 10)
            (`self.ChangeToWhite`)
            (elif (not (== _current_world_state 12))
              (`KismetSystemLibrary.PrintString` "This Shouldn't Happen"))))))))

(fn `ChangeToConcrete`
  (`StaticMeshComponent.SetStaticMesh` (`self.Whitebox_Sphere`) "/Game/GolfGame/Assets/Objects/Sphere/Concrete_Helmets.Concrete_Helmets"))

(fn `ChangeToGrass`
  (`StaticMeshComponent.SetStaticMesh` (`self.Whitebox_Sphere`) "/Game/GolfGame/Assets/Objects/Sphere/Grass_Ball.Grass_Ball"))

(fn `ChangeToIce`
  (`StaticMeshComponent.SetStaticMesh` (`self.Whitebox_Sphere`) "/Game/GolfGame/Assets/Objects/Sphere/Ice_Bush.Ice_Bush"))

(fn `ChangeToSand`
  (`StaticMeshComponent.SetStaticMesh` (`self.Whitebox_Sphere`) "/Game/GolfGame/Assets/Objects/Sphere/Sand_Tires.Sand_Tires"))

(fn `ChangeToWhite`
  (`StaticMeshComponent.SetStaticMesh` (`self.Whitebox_Sphere`) "/Game/GolfGame/Assets/Objects/Sphere/Whitebox_Sphere.Whitebox_Sphere"))

(fn `UserConstructionScript`)