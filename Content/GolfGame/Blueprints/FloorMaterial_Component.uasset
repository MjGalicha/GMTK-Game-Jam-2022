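; Golf game component that reskins the floor meshes it is attached under to match the current world state.
; On BeginPlay it stores its parent components and gives each a dynamic M_AssetPlatform material.
; Tick polls BP_GolfGameMode's ChangeWorldState flag, then maps CurrentWorldState to grass, ice, sand, concrete or white test-level functions.
; Each function swaps material slot 0 on the stored components and prints a joke or debug message.
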(event `self.ReceiveBeginPlay`
  (bind _parents (`self.GetParentComponents`))
  ;[1 1 1] On Initialize - Capture static meshes of parents
  (set `self.Static Mesh` _parents)
  (for _array_element _parents
    (bind _asprimitive_component (cast `PrimitiveComponent` _array_element))
    (`PrimitiveComponent.CreateDynamicMaterialInstance` _asprimitive_component 0 "/Game/StarterContent/Materials/M_AssetPlatform.M_AssetPlatform" "None")))

(event `self.ReceiveTick`
  (params (DeltaSeconds :type "Float (single-precision)"))
  ;[1 1 1] Check if world state has changed, if it has changed, run world state change
  (bind _asbp_golf_game_mode (cast `/Game/GolfGame/Blueprints/BP_GolfGameMode` (`GameplayStatics.GetGameMode`)))
  (if (`/Game/GolfGame/Blueprints/BP_GolfGameMode.Change World State` _asbp_golf_game_mode)
    (`self.Change World State`)))

(event `Change World State`
  ;[1 1 1] Run specific state change function
  (bind _asbp_golf_game_mode (cast `/Game/GolfGame/Blueprints/BP_GolfGameMode` (`GameplayStatics.GetGameMode`)))
  (bind _current_world_state (`/Game/GolfGame/Blueprints/BP_GolfGameMode.Current World State` _asbp_golf_game_mode))
  (if (== _current_world_state 2)
    (`self.ChangeToGrass`)
    (elif (== _current_world_state 4)
      (`self.ChangeToIce`)
      (elif (== _current_world_state 6)
        (`self.ChangeToSand`)
        (elif (== _current_world_state 8)
          (`self.ChangeToConcrete`)
          (elif (== _current_world_state 10)
            (`self.ChangeToWhite`)
            (elif (not (== _current_world_state 12))
              (`KismetSystemLibrary.PrintString` "This Shouldn't Happen"))))))))

(fn `ChangeToConcrete`
  (for _array_element (`self.Static Mesh`)
    (bind _asprimitive_component (cast `PrimitiveComponent` _array_element))
    (`PrimitiveComponent.SetMaterial` _asprimitive_component 0 "/Game/GolfGame/Assets/WorldMats/Concrete/MI_Concrete.MI_Concrete")
    (`KismetSystemLibrary.PrintString` "Fuck yeah, CON-CRETE")))

(fn `ChangeToGrass`
  (for _array_element (`self.Static Mesh`)
    (bind _asprimitive_component (cast `PrimitiveComponent` _array_element))
    (`PrimitiveComponent.SetMaterial` _asprimitive_component 0 "/Game/GolfGame/Assets/WorldMats/Grass/Grass_MAT.Grass_MAT")
    (`KismetSystemLibrary.PrintString` "Your Ass Is Grass")))

(fn `ChangeToIce`
  (for _array_element (`self.Static Mesh`)
    (bind _asprimitive_component (cast `PrimitiveComponent` _array_element))
    (`PrimitiveComponent.SetMaterial` _asprimitive_component 0 "/Game/GolfGame/Assets/WorldMats/Ice/MI_Ice_Graph.MI_Ice_Graph")
    (`KismetSystemLibrary.PrintString` "Ice To Meet You")))

(fn `ChangeToSand`
  (for _array_element (`self.Static Mesh`)
    (bind _asprimitive_component (cast `PrimitiveComponent` _array_element))
    (`PrimitiveComponent.SetMaterial` _asprimitive_component 0 "/Game/GolfGame/Assets/WorldMats/Sand/MI_I_Hate_Sand.MI_I_Hate_Sand")
    (`KismetSystemLibrary.PrintString` "I don't like Sand, It's coarse and rough and irritating and it gets everywhere")))

(fn `ChangeToWhite`
  (for _array_element (`self.Static Mesh`)
    (bind _asprimitive_component (cast `PrimitiveComponent` _array_element))
    (`PrimitiveComponent.SetMaterial` _asprimitive_component 0 "/Game/StarterContent/Materials/M_AssetPlatform.M_AssetPlatform")
    (`KismetSystemLibrary.PrintString` "Test Level")))