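; Floor material controller for the golf game that swaps the surface material on its static mesh.
; Separate functions set element 0 to grass, ice, sand, concrete or a white test platform material, each printing a joke or label on screen.
; BeginPlay creates a dynamic instance of the platform material, but the functions assign fixed materials directly and change only the material.
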(event `self.ReceiveBeginPlay`
  (`PrimitiveComponent.CreateDynamicMaterialInstance` (`self.StaticMesh`) 0 "/Game/StarterContent/Materials/M_AssetPlatform.M_AssetPlatform" "None"))

(fn `ChangeToConcrete`
  (`PrimitiveComponent.SetMaterial` (`self.StaticMesh`) 0 "/Game/GolfGame/Assets/WorldMats/Concrete/MI_Concrete.MI_Concrete")
  (`KismetSystemLibrary.PrintString` "Fuck Yeah, CON-CRETE"))

(fn `ChangeToGrass`
  (`PrimitiveComponent.SetMaterial` (`self.StaticMesh`) 0 "/Game/GolfGame/Assets/WorldMats/Grass/Grass_MAT.Grass_MAT")
  (`KismetSystemLibrary.PrintString` "Your Ass Is Grass"))

(fn `ChangeToIce`
  (`PrimitiveComponent.SetMaterial` (`self.StaticMesh`) 0 "/Game/GolfGame/Assets/WorldMats/Ice/MI_Ice_Graph.MI_Ice_Graph")
  (`KismetSystemLibrary.PrintString` "Ice To Meet You"))

(fn `ChangeToSand`
  (`PrimitiveComponent.SetMaterial` (`self.StaticMesh`) 0 "/Game/GolfGame/Assets/WorldMats/Sand/MI_I_Hate_Sand.MI_I_Hate_Sand")
  (`KismetSystemLibrary.PrintString` "I don't like Sand, It's coarse and rough and irritating and it gets everywhere"))

(fn `ChangeToWhite`
  (`PrimitiveComponent.SetMaterial` (`self.StaticMesh`) 0 "/Game/StarterContent/Materials/M_AssetPlatform.M_AssetPlatform")
  (`KismetSystemLibrary.PrintString` "Test Environment"))

(fn `UserConstructionScript`)