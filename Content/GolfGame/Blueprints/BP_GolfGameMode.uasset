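; Game mode for the golf game that tracks world-state changes, handles winning and advances through levels.
; Tick compares CurrentWorldState to NewWorldState, copies any new value and raises ChangeWorldState, clearing it on the next tick without a change.
; Win shows the victory screen widget, pauses the game and enables the cursor with game-and-UI input.
; LoadNextLevel opens the next numbered level by name, returning to the main menu after the fifth.
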(event `self.ReceiveTick`
  (params (DeltaSeconds :type "Float (single-precision)"))
  (bind _new_world_state (`self.New World State`))
  ;[1 1 1] Check every second and flag if world state has changed
  (if (== (`self.Current World State`) _new_world_state)
    (if (`self.Change World State`)
      (set `self.Change World State` false))
    (else
      (set `self.Current World State` _new_world_state)
      (set `self.Change World State` true))))

(fn `LoadNextLevel`
  (bind _currentlevel (`self.CurrentLevel`))
  (if (>= _currentlevel 5)
    (`GameplayStatics.OpenLevel` "Level_MainMenu")
    (else
      (`GameplayStatics.OpenLevel` (`KismetStringLibrary.Conv_StringToName` (`KismetStringLibrary.Concat_StrStr` "Level_" (`KismetStringLibrary.Conv_IntToString` (+ _currentlevel 1))))))))

(fn `UserConstructionScript`)

(fn `Win`
  (bind _returnvalue (`GameplayStatics.GetPlayerController` 0))
  (bind _returnvalue_2 (`|CreateWidget` "/Game/GolfGame/Blueprints/UI/BP_UI_VICTORY_SCREEEEEEEEEECH.BP_UI_VICTORY_SCREEEEEEEEEECH_C"))
  (`UserWidget.AddToViewport` _returnvalue_2 0)
  (`GameplayStatics.SetGamePaused` true)
  (`WidgetBlueprintLibrary.SetInputMode_GameAndUIEx` _returnvalue null)
  (set `PlayerController.bShowMouseCursor` true _returnvalue))