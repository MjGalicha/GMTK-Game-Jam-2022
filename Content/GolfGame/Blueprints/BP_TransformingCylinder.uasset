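; BP_TransformingCylinder is a golf game prop that changes its mesh to match the current world state.
; Tick polls BP_GolfGameMode's ChangeWorldState flag and, while it is set, branches on CurrentWorldState.
; Helper functions set the static mesh to a grass or ice tree, cactus, traffic cone or plain cylinder.
; One state leaves the mesh unchanged, and unrecognised states print a warning.
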(event `self.ReceiveTick`
  (params (DeltaSeconds :type "Float (single-precision)"))
  ;[1 1 1] Check if world state has changed, if it has changed, run world state change
  (bind _asbp_golf_game_mode (cast `/Game/GolfGame/Blueprints/BP_GolfGameMode` (`GameplayStatics.GetGameMode`)))
  (if (`/Game/GolfGame/Blueprints/BP_GolfGameMode.Change World State` _asbp_golf_game_mode)
    (`self.Change World State`)))

(event `Change World State`
  ;[1 1 1] Run specific state change function
  (bind _asbp_golf_game_mode (cast `/Game/GolfGame/Blueprints/BP_GolfGameMode` (`GameplayStatics.GetGameMode`)))
  (bind _current_world_state (`/Game/GolfGame/Blueprints/BP_GolfGameMode.Current World State` _asbp_golf_game_mode))
  (if (== _current_world_state 2)
    (`self.ChangeToGrass`)
    (elif (== _current_world_state 4)
      (`self.ChangeToIce`)
      (elif (== _current_world_state 6)
        (`self.ChangeToSand`)
        (elif (== _current_world_state 8)
          (`self.ChangeToConcrete`)
          (elif (== _current_world_state 10)
            (`self.ChangeToWhite`)
            (elif (not (== _current_world_state 12))
              (`KismetSystemLibrary.PrintString` "This Shouldn't Happen"))))))))

(fn `ChangeToConcrete`
  (`StaticMeshComponent.SetStaticMesh` (`self.SM_Whitebox_Cylinder`) "/Game/GolfGame/Assets/Objects/Cylinders/SM_Concrete_TrafficCone.SM_Concrete_TrafficCone"))

(fn `ChangeToGrass`
  (`StaticMeshComponent.SetStaticMesh` (`self.SM_Whitebox_Cylinder`) "/Game/GolfGame/Assets/Objects/Cylinders/SM_Grass_Tree.SM_Grass_Tree"))

(fn `ChangeToIce`
  (`StaticMeshComponent.SetStaticMesh` (`self.SM_Whitebox_Cylinder`) "/Game/GolfGame/Assets/Objects/Cylinders/SM_Ice_Tree.SM_Ice_Tree"))

(fn `ChangeToSand`
  (`StaticMeshComponent.SetStaticMesh` (`self.SM_Whitebox_Cylinder`) "/Game/GolfGame/Assets/Objects/Cylinders/SM_Sand_Cactus.SM_Sand_Cactus"))

(fn `ChangeToWhite`
  (`StaticMeshComponent.SetStaticMesh` (`self.SM_Whitebox_Cylinder`) "/Game/GolfGame/Assets/Whitebox_Level/Level_1/SM_Cylinder.SM_Cylinder"))

(fn `UserConstructionScript`)